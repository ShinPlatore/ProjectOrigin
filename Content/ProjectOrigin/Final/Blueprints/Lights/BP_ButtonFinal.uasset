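; BP_ButtonFinal is an interactive button that shows its state through materials and displays a button tutorial prompt to the first-person player.
; Box overlaps track InRange and swap base and collide materials, while ChangeIntoTriggerColor briefly applies a trigger material, plays BoutonPress and restores the range-appropriate one.
; A separate BoxWidget volume creates temporary WBP_Tuto widgets on entry and exit, using delayed fade animations before removing each.
; Two leftover tutorial chains are never run.
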(event OnComponentBeginOverlap(BoxWidget)
  (params (OverlappedComponent :type Primitive%20Component%20Object%20Reference) (OtherActor :type Actor%20Object%20Reference) (OtherComp :type Primitive%20Component%20Object%20Reference) (OtherBodyIndex :type Integer) (bFromSweep :type Boolean) (SweepResult :type Hit%20Result%20Structure%20%28by%20ref%29))
  (Utilities|Casting|CastToBP_FirstPCharacterFinal OtherActor)
  (bind _returnvalue (UserInterface|CreateWidget "/Game/ProjectOrigin/Final/UI/WBP_Tuto.WBP_Tuto_C"))
  (UserInterface|Viewport|AddtoViewport _returnvalue 0)
  (Widget|SetVisibility (Variables|/Game/ProjectOrigin/Final/UI/WBP_Tuto.WBP_Tuto_C|GetText_Crouch _returnvalue) "Hidden")
  (UserInterface|Animation|PlayAnimation _returnvalue (Variables|/Game/ProjectOrigin/Final/UI/WBP_Tuto.WBP_Tuto_C|GetButtonFadeIn _returnvalue) 0.0 1 "Forward" 1.0 false)
  (Widget|SetVisibility (Variables|/Game/ProjectOrigin/Final/UI/WBP_Tuto.WBP_Tuto_C|GetText_Button _returnvalue) "Visible")
  (Utilities|FlowControl|Delay 4.0)
  (UserInterface|Animation|PlayAnimation _returnvalue (Variables|/Game/ProjectOrigin/Final/UI/WBP_Tuto.WBP_Tuto_C|GetButtonFadeOut _returnvalue) 0.0 1 "Forward" 1.0 false)
  (Utilities|FlowControl|Delay 1.0)
  (Widget|SetVisibility (Variables|/Game/ProjectOrigin/Final/UI/WBP_Tuto.WBP_Tuto_C|GetText_Button _returnvalue) "Hidden")
  (Widget|RemovefromParent _returnvalue))

(event OnComponentEndOverlap(BoxWidget)
  (params (OverlappedComponent :type Primitive%20Component%20Object%20Reference) (OtherActor :type Actor%20Object%20Reference) (OtherComp :type Primitive%20Component%20Object%20Reference) (OtherBodyIndex :type Integer))
  (Utilities|Casting|CastToBP_FirstPCharacterFinal OtherActor)
  (bind _returnvalue (UserInterface|CreateWidget "/Game/ProjectOrigin/Final/UI/WBP_Tuto.WBP_Tuto_C"))
  (UserInterface|Viewport|AddtoViewport _returnvalue 0)
  (Widget|SetVisibility (Variables|/Game/ProjectOrigin/Final/UI/WBP_Tuto.WBP_Tuto_C|GetText_Crouch _returnvalue) "Hidden")
  (UserInterface|Animation|PlayAnimation _returnvalue (Variables|/Game/ProjectOrigin/Final/UI/WBP_Tuto.WBP_Tuto_C|GetButtonFadeOut _returnvalue) 0.0 1 "Forward" 1.0 false)
  (Utilities|FlowControl|Delay 0.2)
  (Widget|SetVisibility (Variables|/Game/ProjectOrigin/Final/UI/WBP_Tuto.WBP_Tuto_C|GetText_Sprint _returnvalue) "Hidden")
  (Widget|RemovefromParent _returnvalue))

(event OnComponentBeginOverlap(Box)
  (params (OverlappedComponent :type Primitive%20Component%20Object%20Reference) (OtherActor :type Actor%20Object%20Reference) (OtherComp :type Primitive%20Component%20Object%20Reference) (OtherBodyIndex :type Integer) (bFromSweep :type Boolean) (SweepResult :type Hit%20Result%20Structure%20%28by%20ref%29))
  ;[0 0 0 1 25] Button Behavior
  (Utilities|Casting|CastToBP_FirstPCharacterFinal OtherActor)
  (Variables|Default|SetInRange true)
  (Rendering|Material|SetMaterial (Variables|Default|GetCube) 0 "/Game/ProjectOrigin/Patrick/Mat/M_ButtonCollide.M_ButtonCollide"))

(event OnComponentEndOverlap(Box)
  (params (OverlappedComponent :type Primitive%20Component%20Object%20Reference) (OtherActor :type Actor%20Object%20Reference) (OtherComp :type Primitive%20Component%20Object%20Reference) (OtherBodyIndex :type Integer))
  ;[0 0 0 1 25] Button Behavior
  (Utilities|Casting|CastToBP_FirstPCharacterFinal OtherActor)
  (Variables|Default|SetInRange false)
  (Rendering|Material|SetMaterial (Variables|Default|GetCube) 0 "/Game/ProjectOrigin/Patrick/Mat/M_ButtonBase.M_ButtonBase"))

(event Custom|ChangeIntoTriggerColor
  (bind _cube (Variables|Default|GetCube))
  ;[0 0 0 1 25] Button Behavior
  (Rendering|Material|SetMaterial (Variables|Default|GetCube) 0 "/Game/ProjectOrigin/Patrick/Mat/M_ButtonTrigger.M_ButtonTrigger")
  (Audio|Components|Audio|Play (Variables|Default|GetBoutonPress) 0.0)
  (Utilities|FlowControl|Delay 0.5)
  (if (Variables|Default|GetInRange)
    (Rendering|Material|SetMaterial _cube 0 "/Game/ProjectOrigin/Patrick/Mat/M_ButtonCollide.M_ButtonCollide")
    (else
      (Rendering|Material|SetMaterial _cube 0 "/Game/ProjectOrigin/Patrick/Mat/M_ButtonBase.M_ButtonBase"))))

(event EventBeginPlay
  (Audio|Components|Audio|Stop (Variables|Default|GetBoutonPress)))

(fn ConstructionScript)