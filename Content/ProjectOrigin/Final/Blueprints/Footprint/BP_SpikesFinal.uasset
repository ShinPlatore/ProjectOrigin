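; BP_SpikesFinal is a spike trap with a disappearing plane that kills the first-person character (BP_FirstPCharacterVirgile).
; When the character overlaps Box, the Plane is hidden and loses its collision.
; Overlapping Box1 destroys the character, then after a short delay shows the Plane again with physics-only collision rather than query-and-physics.
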(event OnComponentBeginOverlap(Box)
  (params (OverlappedComponent :type Primitive%20Component%20Object%20Reference) (OtherActor :type Actor%20Object%20Reference) (OtherComp :type Primitive%20Component%20Object%20Reference) (OtherBodyIndex :type Integer) (bFromSweep :type Boolean) (SweepResult :type Hit%20Result%20Structure%20%28by%20ref%29))
  (bind _plane (Variables|Default|GetPlane))
  (Utilities|Casting|CastToBP_FirstPCharacterVirgile OtherActor)
  (Development|SetHiddeninGame _plane true false)
  (Collision|SetCollisionEnabled _plane "NoCollision"))

(event OnComponentBeginOverlap(Box1)
  (params (OverlappedComponent :type Primitive%20Component%20Object%20Reference) (OtherActor :type Actor%20Object%20Reference) (OtherComp :type Primitive%20Component%20Object%20Reference) (OtherBodyIndex :type Integer) (bFromSweep :type Boolean) (SweepResult :type Hit%20Result%20Structure%20%28by%20ref%29))
  (bind _plane (Variables|Default|GetPlane))
  (bind _asbp_first_pcharacter_virgile (Utilities|Casting|CastToBP_FirstPCharacterVirgile OtherActor))
  (Actor|DestroyActor _asbp_first_pcharacter_virgile)
  (Utilities|FlowControl|Delay 2.0)
  (Development|SetHiddeninGame _plane false false)
  (Collision|SetCollisionEnabled _plane "PhysicsOnly"))

(fn ConstructionScript)