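; Trigger volume that raises the referenced lights actor's Cube toward a fixed height when the first-person player character enters.
; An Elevate timeline plays on overlap and reverses on exit, lerping from the Cube's current Z each update, so reversing does not lower it.
; A Reset event restores the Cube's stored relative transform.
; Disconnected leftover logic covers health-based resets and respawn placement.
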(event OnComponentBeginOverlap(Box)
  (params (OverlappedComponent :type Primitive%20Component%20Object%20Reference) (OtherActor :type Actor%20Object%20Reference) (OtherComp :type Primitive%20Component%20Object%20Reference) (OtherBodyIndex :type Integer) (bFromSweep :type Boolean) (SweepResult :type Hit%20Result%20Structure%20%28by%20ref%29))
  (bind _lightsref (Variables|Default|GetLightsREF))
  (bind _cube (Variables|/Game/ProjectOrigin/Final/Blueprints/Footprint/BP_LightsFinal.BP_LightsFinal_C|GetCube _lightsref))
  (bind _relativelocation (Variables|/Script/Engine.SceneComponent|GetRelativeLocation _cube))
  (Utilities|Casting|CastToBP_FirstPCharacterFinal OtherActor)
  (bind _delta (Timeline|Elevate Play)
    (:Update
      (Transformation|SetRelativeLocation (Variables|/Game/ProjectOrigin/Final/Blueprints/Footprint/BP_LightsFinal.BP_LightsFinal_C|GetCube (Variables|Default|GetLightsREF)) (Math|Vector|Lerp(Vector) (Math|Vector|MakeVector (.x _relativelocation) (.y _relativelocation) (.z _relativelocation)) (Math|Vector|MakeVector (.x _relativelocation) (.y _relativelocation) 6e+02) _delta) false false))))

(event OnComponentEndOverlap(Box)
  (params (OverlappedComponent :type Primitive%20Component%20Object%20Reference) (OtherActor :type Actor%20Object%20Reference) (OtherComp :type Primitive%20Component%20Object%20Reference) (OtherBodyIndex :type Integer))
  (bind _lightsref (Variables|Default|GetLightsREF))
  (bind _cube (Variables|/Game/ProjectOrigin/Final/Blueprints/Footprint/BP_LightsFinal.BP_LightsFinal_C|GetCube _lightsref))
  (bind _relativelocation (Variables|/Script/Engine.SceneComponent|GetRelativeLocation _cube))
  (Utilities|Casting|CastToBP_FirstPCharacterFinal OtherActor)
  (bind _delta (Timeline|Elevate Reverse)
    (:Update
      (Transformation|SetRelativeLocation (Variables|/Game/ProjectOrigin/Final/Blueprints/Footprint/BP_LightsFinal.BP_LightsFinal_C|GetCube (Variables|Default|GetLightsREF)) (Math|Vector|Lerp(Vector) (Math|Vector|MakeVector (.x _relativelocation) (.y _relativelocation) (.z _relativelocation)) (Math|Vector|MakeVector (.x _relativelocation) (.y _relativelocation) 6e+02) _delta) false false))))

(event Custom|Reset
  (Transformation|SetRelativeTransform (Variables|/Game/ProjectOrigin/Final/Blueprints/Footprint/BP_LightsFinal.BP_LightsFinal_C|GetCube (Variables|Default|GetLightsREF)) (Variables|Default|GetLightsCubeREF) false false))

(event EventTick
  (params (DeltaSeconds :type Float%20%28single-precision%29)))

(event EventBeginPlay)

(fn ConstructionScript)