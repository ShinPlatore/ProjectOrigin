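; BP_SucceedFinal is a box trigger that marks the footprint challenge as succeeded when the BP_FirstPCharacterVirgile character enters it.
; BeginPlay clears HasSucceed on the player character and copies it to HasSucceededFootPrint on the BP_SpawnPointsFinal game instance.
; Overlapping the box sets both flags to true and prints the game instance value in green as debug output.
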(event OnComponentBeginOverlap(Box)
  (params (OverlappedComponent :type Primitive%20Component%20Object%20Reference) (OtherActor :type Actor%20Object%20Reference) (OtherComp :type Primitive%20Component%20Object%20Reference) (OtherBodyIndex :type Integer) (bFromSweep :type Boolean) (SweepResult :type Hit%20Result%20Structure%20%28by%20ref%29))
  (bind _asbp_first_pcharacter_virgile (Utilities|Casting|CastToBP_FirstPCharacterVirgile OtherActor))
  (bind _output_get (Variables|/Game/ProjectOrigin/Virgile/Blueprints/Character/BP_FirstPCharacterVirgile.BP_FirstPCharacterVirgile_C|SethasSucceed _asbp_first_pcharacter_virgile true))
  (bind _asbp_spawn_points (Utilities|Casting|CastToBP_SpawnPointsFinal (Game|GetGameInstance)))
  (bind _output_get_2 (Variables|/Game/ProjectOrigin/Final/Blueprints/BP_SpawnPointsFinal.BP_SpawnPointsFinal_C|SethasSucceededFootPrint _asbp_spawn_points _output_get))
  (Development|PrintString (Utilities|String|ToString(Boolean) _output_get_2) true true "(R=0.000000,G=1.000000,B=0.271407,A=1.000000)"))

(event EventBeginPlay
  (bind _asbp_first_pcharacter_virgile (Utilities|Casting|CastToBP_FirstPCharacterVirgile (Game|GetPlayerCharacter 0)))
  (bind _output_get (Variables|/Game/ProjectOrigin/Virgile/Blueprints/Character/BP_FirstPCharacterVirgile.BP_FirstPCharacterVirgile_C|SethasSucceed _asbp_first_pcharacter_virgile false))
  (bind _asbp_spawn_points (Utilities|Casting|CastToBP_SpawnPointsFinal (Game|GetGameInstance)))
  (Variables|/Game/ProjectOrigin/Final/Blueprints/BP_SpawnPointsFinal.BP_SpawnPointsFinal_C|SethasSucceededFootPrint _asbp_spawn_points _output_get))

(fn ConstructionScript)