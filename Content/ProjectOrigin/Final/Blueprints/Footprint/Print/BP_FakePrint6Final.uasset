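; BP_FakePrint6Final is a fake footprint actor that is visible only while the player has night vision.
; It hides its Plane and StaticMesh components on BeginPlay.
; Every Tick calls Display, which casts the player character to BP_FirstPCharacterFinal and sets both components' visibility from HasNightVision by polling rather than responding to an event.
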(event Custom|Display
  (bind _asbp_first_pcharacter_final (Utilities|Casting|CastToBP_FirstPCharacterFinal (Game|GetPlayerCharacter 0)))
  (if (== (Variables|/Game/ProjectOrigin/Final/Blueprints/Character/BP_FirstPCharacterFinal.BP_FirstPCharacterFinal_C|GethasNightVision _asbp_first_pcharacter_final) true)
    (Development|SetHiddeninGame (Variables|Default|GetPlane) false false)
    (else
      (Development|SetHiddeninGame (Variables|Default|GetPlane) true false))))

(event EventBeginPlay
  (Development|SetHiddeninGame (Variables|Default|GetPlane) true false))

(event EventTick
  (params (DeltaSeconds :type Float%20%28single-precision%29))
  (CallFunction|Display))

(fn ConstructionScript)