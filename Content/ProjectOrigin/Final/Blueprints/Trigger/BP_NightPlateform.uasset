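; Timed platform Blueprint with a floor mesh and a wall mesh that each blink in and out of existence every second.
; Tick accumulates time and uses whole-second parity to toggle visibility and collision, reapplying the state every frame.
; IsPair and IsLateralPair set each mesh's phase and its BeginPlay material, allowing alternating patterns.
; SetNightStatus switches the platform mesh's Emissive parameter but is not called within this graph.
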(event EventBeginPlay
  (bind _staticmesh (Variables|Default|GetStaticMesh))
  (bind _wallmesh (Variables|Default|GetWallMesh))
  (Utilities|FlowControl|Sequence
    (:then_0
      (if (Variables|Default|GetIsPair)
        (Rendering|Material|SetMaterial _staticmesh 0 "/AnimationSharing/AnimSharingBlue.AnimSharingBlue")
        (else
          (Rendering|Material|SetMaterial _staticmesh 0 "/AnimationSharing/AnimSharingRed.AnimSharingRed"))))
    (:then_1
      (if (Variables|Default|GetIsLateralPair)
        (Rendering|Material|SetMaterial _wallmesh 0 "/AnimationSharing/AnimSharingGreen.AnimSharingGreen")
        (else
          (Rendering|Material|SetMaterial _wallmesh 0 "/Engine/EditorResources/FieldNodes/_Resources/M_FieldRadiusPreview.M_FieldRadiusPreview"))))))

(event EventTick
  (params (DeltaSeconds :type Float%20%28single-precision%29))
  (bind _output_get (Variables|Default|Settimer (+ DeltaSeconds (Variables|Default|Gettimer))))
  (bind _output_get_2 (Variables|Default|SetTruncate (Math|Float|Truncate _output_get)))
  (bind _output_get_3 (Variables|Default|SetModulo (Math|Integer|%(Integer) _output_get_2 2)))
  (if (Variables|Default|GetIsPair)
    (if (== _output_get_3 0)
      (CallFunction|SetMeshtoVoid)
      (else
        (CallFunction|SetMeshtoSolid)))
    (elif (== _output_get_3 0)
      (CallFunction|SetMeshtoSolid)
      (else
        (CallFunction|SetMeshtoVoid))))
  (if (Variables|Default|GetIsLateralPair)
    (if (== (Variables|Default|GetModulo) 0)
      (CallFunction|SetWallMesh)
      (else
        (CallFunction|SetWallMeshVoid)))
    (elif (== (Variables|Default|GetModulo) 0)
      (CallFunction|SetWallMeshVoid)
      (else
        (CallFunction|SetWallMesh)))))

(fn ConstructionScript)

(fn SetNightStatus
  (params (NewParam :type Boolean))
  (bind _staticmesh (Variables|Default|GetStaticMesh))
  (if NewParam
    (Rendering|Material|SetScalarParameterValueonMaterials _staticmesh "Emissive" 1.0)
    (else
      (Rendering|Material|SetScalarParameterValueonMaterials _staticmesh "Emissive" 0.0))))

(fn SetMeshtoVoid
  (Rendering|SetVisibility (Variables|Default|GetStaticMesh) false false)
  (Collision|SetCollisionEnabled (Variables|Default|GetStaticMesh) "NoCollision"))

(fn SetMeshtoSolid
  (Rendering|SetVisibility (Variables|Default|GetStaticMesh) true false)
  (Collision|SetCollisionEnabled (Variables|Default|GetStaticMesh) "QueryAndPhysics"))

(fn SetWallMesh
  (Rendering|SetVisibility (Variables|Default|GetWallMesh) true false)
  (Collision|SetCollisionEnabled (Variables|Default|GetWallMesh) "QueryAndPhysics"))

(fn SetWallMeshVoid
  (Rendering|SetVisibility (Variables|Default|GetWallMesh) false false)
  (Collision|SetCollisionEnabled (Variables|Default|GetWallMesh) "NoCollision"))