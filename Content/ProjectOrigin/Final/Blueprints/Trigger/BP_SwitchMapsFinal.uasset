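; Trigger box that switches maps between the Temple and Footprint levels when the first-person character overlaps it.
; If the character has succeeded, it fades to black, stores its spawn point in the BP_SpawnPointsFinal game instance and opens TempleFinal after a short delay.
; Otherwise, it destroys the character if the game instance flags Footprint as already visited, or fades out and opens FootprintFinal if not.
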(event OnComponentBeginOverlap(Box)
  (params (OverlappedComponent :type Primitive%20Component%20Object%20Reference) (OtherActor :type Actor%20Object%20Reference) (OtherComp :type Primitive%20Component%20Object%20Reference) (OtherBodyIndex :type Integer) (bFromSweep :type Boolean) (SweepResult :type Hit%20Result%20Structure%20%28by%20ref%29))
  (bind _asbp_first_pcharacter_final (Utilities|Casting|CastToBP_FirstPCharacterFinal OtherActor))
  (if (== (Variables|/Game/ProjectOrigin/Final/Blueprints/Character/BP_FirstPCharacterFinal.BP_FirstPCharacterFinal_C|GethasSucceed _asbp_first_pcharacter_final) true)
    (bind _returnvalue (UserInterface|CreateWidget "/Game/ProjectOrigin/Final/UI/WBP_BlackFadeFinal.WBP_BlackFadeFinal_C"))
    (UserInterface|Viewport|AddtoViewport _returnvalue 0)
    (UserInterface|Animation|PlayAnimation _returnvalue (Variables|/Game/ProjectOrigin/Final/UI/WBP_BlackFadeFinal.WBP_BlackFadeFinal_C|GetFadeIn _returnvalue) 0.0 1 "Forward" 1.0 false)
    (Utilities|FlowControl|Delay 1.0)
    (bind _asbp_spawn_points_final (Utilities|Casting|CastToBP_SpawnPointsFinal (Game|GetGameInstance)))
    (Variables|/Game/ProjectOrigin/Final/Blueprints/BP_SpawnPointsFinal.BP_SpawnPointsFinal_C|SetSpawnPointFootPrint _asbp_spawn_points_final (Variables|Default|GetSpawnPoint))
    (Game|OpenLevel(byObjectReference) "/Game/ProjectOrigin/Final/Maps/TempleFinal.TempleFinal")
    (elif (== (Variables|/Game/ProjectOrigin/Final/Blueprints/BP_SpawnPointsFinal.BP_SpawnPointsFinal_C|GethasBeenFootprint (.AsBP%20Spawn%20Points%20Final (Utilities|Casting|CastToBP_SpawnPointsFinal (Game|GetGameInstance)))) true)
      (Actor|DestroyActor _asbp_first_pcharacter_final)
      (else
        (bind _returnvalue_2 (UserInterface|CreateWidget "/Game/ProjectOrigin/Final/UI/WBP_BlackFadeFinal.WBP_BlackFadeFinal_C"))
        (UserInterface|Viewport|AddtoViewport _returnvalue_2 0)
        (UserInterface|Animation|PlayAnimation _returnvalue_2 (Variables|/Game/ProjectOrigin/Final/UI/WBP_BlackFadeFinal.WBP_BlackFadeFinal_C|GetFadeIn _returnvalue_2) 0.0 1 "Forward" 1.0 false)
        (Utilities|FlowControl|Delay 1.0)
        (Game|OpenLevel(byObjectReference) "/Game/ProjectOrigin/Final/Maps/FootprintFinal.FootprintFinal")))))

(fn ConstructionScript)