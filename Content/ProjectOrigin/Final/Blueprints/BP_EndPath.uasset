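; End-path actor whose ten brick meshes slide into place as the first-person character advances through it.
; Five trigger boxes each play two timelines, lerping a pair of bricks from their current relative locations toward End markers.
; EndBox overlap destroys the character and sets IsDead.
; Tick polls that flag and snaps bricks back to stored Brick locations, clearing it without rewinding the timelines.
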(event OnComponentBeginOverlap(Box)
  (params (OverlappedComponent :type Primitive%20Component%20Object%20Reference) (OtherActor :type Actor%20Object%20Reference) (OtherComp :type Primitive%20Component%20Object%20Reference) (OtherBodyIndex :type Integer) (bFromSweep :type Boolean) (SweepResult :type Hit%20Result%20Structure%20%28by%20ref%29))
  (Utilities|Casting|CastToBP_FirstPCharacterFinal OtherActor)
  (Utilities|FlowControl|Sequence
    (:then_0
      (bind _newtrack_0 (Timeline|Timeline Play)
        (:Update
          (CallFunction|SM _newtrack_0))))
    (:then_1
      (bind _newtrack_0_2 (Timeline|Timeline_0 Play)
        (:Update
          (CallFunction|SM01 _newtrack_0_2))))))

(event OnComponentBeginOverlap(EndBox)
  (params (OverlappedComponent :type Primitive%20Component%20Object%20Reference) (OtherActor :type Actor%20Object%20Reference) (OtherComp :type Primitive%20Component%20Object%20Reference) (OtherBodyIndex :type Integer) (bFromSweep :type Boolean) (SweepResult :type Hit%20Result%20Structure%20%28by%20ref%29))
  (bind _asbp_first_pcharacter_final (Utilities|Casting|CastToBP_FirstPCharacterFinal OtherActor))
  (Variables|Default|SetisDead true)
  (Actor|DestroyActor _asbp_first_pcharacter_final))

(event OnComponentBeginOverlap(Box1)
  (params (OverlappedComponent :type Primitive%20Component%20Object%20Reference) (OtherActor :type Actor%20Object%20Reference) (OtherComp :type Primitive%20Component%20Object%20Reference) (OtherBodyIndex :type Integer) (bFromSweep :type Boolean) (SweepResult :type Hit%20Result%20Structure%20%28by%20ref%29))
  (Utilities|Casting|CastToBP_FirstPCharacterFinal OtherActor)
  (Utilities|FlowControl|Sequence
    (:then_0
      (bind _newtrack_0 (Timeline|Timeline_1 Play)
        (:Update
          (CallFunction|SM02 _newtrack_0))))
    (:then_1
      (bind _newtrack_0_2 (Timeline|Timeline_2 Play)
        (:Update
          (CallFunction|SM03 _newtrack_0_2))))))

(event OnComponentBeginOverlap(Box2)
  (params (OverlappedComponent :type Primitive%20Component%20Object%20Reference) (OtherActor :type Actor%20Object%20Reference) (OtherComp :type Primitive%20Component%20Object%20Reference) (OtherBodyIndex :type Integer) (bFromSweep :type Boolean) (SweepResult :type Hit%20Result%20Structure%20%28by%20ref%29))
  (Utilities|Casting|CastToBP_FirstPCharacterFinal OtherActor)
  (Utilities|FlowControl|Sequence
    (:then_0
      (bind _newtrack_0 (Timeline|Timeline_3 Play)
        (:Update
          (CallFunction|SM04 _newtrack_0))))
    (:then_1
      (bind _newtrack_0_2 (Timeline|Timeline_4 Play)
        (:Update
          (CallFunction|SM05 _newtrack_0_2))))))

(event OnComponentBeginOverlap(Box3)
  (params (OverlappedComponent :type Primitive%20Component%20Object%20Reference) (OtherActor :type Actor%20Object%20Reference) (OtherComp :type Primitive%20Component%20Object%20Reference) (OtherBodyIndex :type Integer) (bFromSweep :type Boolean) (SweepResult :type Hit%20Result%20Structure%20%28by%20ref%29))
  (Utilities|Casting|CastToBP_FirstPCharacterFinal OtherActor)
  (Utilities|FlowControl|Sequence
    (:then_0
      (bind _newtrack_0 (Timeline|Timeline_5 Play)
        (:Update
          (CallFunction|SM06 _newtrack_0))))
    (:then_1
      (bind _newtrack_0_2 (Timeline|Timeline_6 Play)
        (:Update
          (CallFunction|SM07 _newtrack_0_2))))))

(event OnComponentBeginOverlap(Box4)
  (params (OverlappedComponent :type Primitive%20Component%20Object%20Reference) (OtherActor :type Actor%20Object%20Reference) (OtherComp :type Primitive%20Component%20Object%20Reference) (OtherBodyIndex :type Integer) (bFromSweep :type Boolean) (SweepResult :type Hit%20Result%20Structure%20%28by%20ref%29))
  (Utilities|Casting|CastToBP_FirstPCharacterFinal OtherActor)
  (Utilities|FlowControl|Sequence
    (:then_0
      (bind _newtrack_0 (Timeline|Timeline_7 Play)
        (:Update
          (CallFunction|SM08 _newtrack_0))))
    (:then_1
      (bind _newtrack_0_2 (Timeline|Timeline_8 Play)
        (:Update
          (CallFunction|SM09 _newtrack_0_2))))))

(event Custom|Reset
  (Transformation|SetRelativeLocation (Variables|Default|GetStaticMesh) (Variables|Default|GetBrick) false false)
  (Transformation|SetRelativeLocation (Variables|Default|GetStaticMesh1) (Variables|Default|GetBrick1) false false)
  (Transformation|SetRelativeLocation (Variables|Default|GetStaticMesh2) (Variables|Default|GetBrick2) false false)
  (Transformation|SetRelativeLocation (Variables|Default|GetStaticMesh3) (Variables|Default|GetBrick3) false false)
  (Transformation|SetRelativeLocation (Variables|Default|GetStaticMesh4) (Variables|Default|GetBrick4) false false)
  (Transformation|SetRelativeLocation (Variables|Default|GetStaticMesh5) (Variables|Default|GetBrick5) false false)
  (Transformation|SetRelativeLocation (Variables|Default|GetStaticMesh6) (Variables|Default|GetBrick6) false false)
  (Transformation|SetRelativeLocation (Variables|Default|GetStaticMesh7) (Variables|Default|GetBrick7) false false)
  (Transformation|SetRelativeLocation (Variables|Default|GetStaticMesh8) (Variables|Default|GetBrick8) false false)
  (Transformation|SetRelativeLocation (Variables|Default|GetStaticMesh9) (Variables|Default|GetBrick9) false false)
  (Variables|Default|SetisDead false))

(event EventBeginPlay
  (Variables|Default|SetisDead false))

(event EventTick
  (params (DeltaSeconds :type Float%20%28single-precision%29))
  (if (== (Variables|Default|GetisDead) true)
    (CallFunction|Reset)))

(fn ConstructionScript)

(fn SM
  (params (Alpha :type Float%20%28single-precision%29))
  (Transformation|SetRelativeLocation (Variables|Default|GetStaticMesh) (Math|Vector|Lerp(Vector) (Variables|/Script/Engine.SceneComponent|GetRelativeLocation (Variables|Default|GetStaticMesh)) (Variables|/Script/Engine.SceneComponent|GetRelativeLocation (Variables|Default|GetEnd)) Alpha) false false))

(fn SM01
  (params (Alpha :type Float%20%28single-precision%29))
  (Transformation|SetRelativeLocation (Variables|Default|GetStaticMesh1) (Math|Vector|Lerp(Vector) (Variables|/Script/Engine.SceneComponent|GetRelativeLocation (Variables|Default|GetStaticMesh1)) (Variables|/Script/Engine.SceneComponent|GetRelativeLocation (Variables|Default|GetEnd1)) Alpha) false false))

(fn SM02
  (params (Alpha :type Float%20%28single-precision%29))
  (Transformation|SetRelativeLocation (Variables|Default|GetStaticMesh2) (Math|Vector|Lerp(Vector) (Variables|/Script/Engine.SceneComponent|GetRelativeLocation (Variables|Default|GetStaticMesh2)) (Variables|/Script/Engine.SceneComponent|GetRelativeLocation (Variables|Default|GetEnd2)) Alpha) false false))

(fn SM03
  (params (Alpha :type Float%20%28single-precision%29))
  (Transformation|SetRelativeLocation (Variables|Default|GetStaticMesh3) (Math|Vector|Lerp(Vector) (Variables|/Script/Engine.SceneComponent|GetRelativeLocation (Variables|Default|GetStaticMesh3)) (Variables|/Script/Engine.SceneComponent|GetRelativeLocation (Variables|Default|GetEnd3)) Alpha) false false))

(fn SM04
  (params (Alpha :type Float%20%28single-precision%29))
  (Transformation|SetRelativeLocation (Variables|Default|GetStaticMesh4) (Math|Vector|Lerp(Vector) (Variables|/Script/Engine.SceneComponent|GetRelativeLocation (Variables|Default|GetStaticMesh4)) (Variables|/Script/Engine.SceneComponent|GetRelativeLocation (Variables|Default|GetEnd4)) Alpha) false false))

(fn SM05
  (params (Alpha :type Float%20%28single-precision%29))
  (Transformation|SetRelativeLocation (Variables|Default|GetStaticMesh5) (Math|Vector|Lerp(Vector) (Variables|/Script/Engine.SceneComponent|GetRelativeLocation (Variables|Default|GetStaticMesh5)) (Variables|/Script/Engine.SceneComponent|GetRelativeLocation (Variables|Default|GetEnd5)) Alpha) false false))

(fn SM06
  (params (Alpha :type Float%20%28single-precision%29))
  (Transformation|SetRelativeLocation (Variables|Default|GetStaticMesh6) (Math|Vector|Lerp(Vector) (Variables|/Script/Engine.SceneComponent|GetRelativeLocation (Variables|Default|GetStaticMesh6)) (Variables|/Script/Engine.SceneComponent|GetRelativeLocation (Variables|Default|GetEnd6)) Alpha) false false))

(fn SM07
  (params (Alpha :type Float%20%28single-precision%29))
  (Transformation|SetRelativeLocation (Variables|Default|GetStaticMesh7) (Math|Vector|Lerp(Vector) (Variables|/Script/Engine.SceneComponent|GetRelativeLocation (Variables|Default|GetStaticMesh7)) (Variables|/Script/Engine.SceneComponent|GetRelativeLocation (Variables|Default|GetEnd7)) Alpha) false false))

(fn SM08
  (params (Alpha :type Float%20%28single-precision%29))
  (Transformation|SetRelativeLocation (Variables|Default|GetStaticMesh8) (Math|Vector|Lerp(Vector) (Variables|/Script/Engine.SceneComponent|GetRelativeLocation (Variables|Default|GetStaticMesh8)) (Variables|/Script/Engine.SceneComponent|GetRelativeLocation (Variables|Default|GetEnd8)) Alpha) false false))

(fn SM09
  (params (Alpha :type Float%20%28single-precision%29))
  (Transformation|SetRelativeLocation (Variables|Default|GetStaticMesh9) (Math|Vector|Lerp(Vector) (Variables|/Script/Engine.SceneComponent|GetRelativeLocation (Variables|Default|GetStaticMesh9)) (Variables|/Script/Engine.SceneComponent|GetRelativeLocation (Variables|Default|GetEnd9)) Alpha) false false))