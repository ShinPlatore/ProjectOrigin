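; BP_ArtefactFinal is an artefact actor that scripts the transition played when a puzzle ends.
; EndPuzzleTransition fades the screen through the BlackFade on BP_FirstPCharacterFinal, moves the player to TPPosRef, calls a still-empty ShowCinematic stub, then fades again.
; FadeInFadeOut checks FadeIn first, so both calls here only trigger FadeOn and never FadeOff.
; ValidatePuzzleEnd only destroys the actor, despite its comment outlining a longer sequence.
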(event Custom|EndPuzzleTransition
  ;[1 1 1] FadeIn / TP (Door) / FadeOut /Cinematic/ FadeIn_Out / Closing Door / VFX Visibility On
  (CallFunction|FadeinFadeOut "NewEnumerator0" true false)
  (CallFunction|TPCharacter "NewEnumerator0")
  (CallFunction|ShowCinematic "NewEnumerator0")
  (CallFunction|FadeinFadeOut "NewEnumerator0" true true))

(fn ConstructionScript)

(fn ValidatePuzzleEnd
  ;[1 1 1] FadeIn / TP (Door) / FadeOut /FadeIn_Out /Cinematic/ FadeIn_Out / Closing Door / VFX Visibility On
  (Actor|DestroyActor))

(fn ShowCinematic
  (params (PuzzleState :type EPuzzleStates%20Enum :default "NewEnumerator0")))

(fn TPCharacter
  (params (PuzzleState :type EPuzzleStates%20Enum :default "NewEnumerator0"))
  (Transformation|SetActorLocation (Game|GetPlayerCharacter 0) (Transformation|GetActorLocation (Variables|Default|GetTPPosRef)) false false))

(fn FadeinFadeOut
  (params (PuzzleState :type EPuzzleStates%20Enum :default "NewEnumerator0") (FadeIn :type Boolean) (FadeOut :type Boolean))
  (bind _asbp_first_pcharacter_final (Utilities|Casting|CastToBP_FirstPCharacterFinal (Game|GetPlayerCharacter 0)))
  (if FadeIn
    (Default|Fadeon (Variables|/Game/ProjectOrigin/Final/Blueprints/Character/BP_FirstPCharacterFinal.BP_FirstPCharacterFinal_C|GetBlackFade _asbp_first_pcharacter_final))
    (elif FadeOut
      (Default|FadeOff (Variables|/Game/ProjectOrigin/Final/Blueprints/Character/BP_FirstPCharacterFinal.BP_FirstPCharacterFinal_C|GetBlackFade _asbp_first_pcharacter_final)))))