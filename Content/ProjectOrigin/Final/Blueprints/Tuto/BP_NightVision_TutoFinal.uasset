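; Tutorial trigger that shows the night vision hint when the first-person player character enters its box.
; On overlap, if HasBeenDisplayed is false, it creates a WBP_Tuto widget, fades in only the night vision text, then fades it out and removes it after timed delays.
; Leaving the box briefly plays the fade-out on a separate new widget, leaving the stored one untouched.
; HasBeenDisplayed is never set here.
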(event OnComponentBeginOverlap(Box)
  (params (OverlappedComponent :type Primitive%20Component%20Object%20Reference) (OtherActor :type Actor%20Object%20Reference) (OtherComp :type Primitive%20Component%20Object%20Reference) (OtherBodyIndex :type Integer) (bFromSweep :type Boolean) (SweepResult :type Hit%20Result%20Structure%20%28by%20ref%29))
  (Utilities|Casting|CastToBP_FirstPCharacterFinal OtherActor)
  (if (== (Variables|Default|GethasBeenDisplayed) false)
    (bind _returnvalue (UserInterface|CreateWidget "/Game/ProjectOrigin/Final/UI/WBP_Tuto.WBP_Tuto_C"))
    (bind _output_get (Variables|Default|SetTutoREF _returnvalue))
    (UserInterface|Viewport|AddtoViewport _output_get 0)
    (Widget|SetVisibility (Variables|/Game/ProjectOrigin/Final/UI/WBP_Tuto.WBP_Tuto_C|GetText_Crouch _output_get) "Hidden")
    (UserInterface|Animation|PlayAnimation _output_get (Variables|/Game/ProjectOrigin/Final/UI/WBP_Tuto.WBP_Tuto_C|GetNightVisionFadeIn _output_get) 0.0 1 "Forward" 1.0 false)
    (Widget|SetVisibility (Variables|/Game/ProjectOrigin/Final/UI/WBP_Tuto.WBP_Tuto_C|GetText_NightVision _output_get) "Visible")
    (Utilities|FlowControl|Delay 4.0)
    (UserInterface|Animation|PlayAnimation _output_get (Variables|/Game/ProjectOrigin/Final/UI/WBP_Tuto.WBP_Tuto_C|GetNightVisionFadeOut _output_get) 0.0 1 "Forward" 1.0 false)
    (Utilities|FlowControl|Delay 1.0)
    (Widget|SetVisibility (Variables|/Game/ProjectOrigin/Final/UI/WBP_Tuto.WBP_Tuto_C|GetText_NightVision _output_get) "Hidden")
    (Widget|RemovefromParent _output_get)))

(event OnComponentEndOverlap(Box)
  (params (OverlappedComponent :type Primitive%20Component%20Object%20Reference) (OtherActor :type Actor%20Object%20Reference) (OtherComp :type Primitive%20Component%20Object%20Reference) (OtherBodyIndex :type Integer))
  (Utilities|Casting|CastToBP_FirstPCharacterFinal OtherActor)
  (bind _returnvalue (UserInterface|CreateWidget "/Game/ProjectOrigin/Final/UI/WBP_Tuto.WBP_Tuto_C"))
  (UserInterface|Viewport|AddtoViewport _returnvalue 0)
  (Widget|SetVisibility (Variables|/Game/ProjectOrigin/Final/UI/WBP_Tuto.WBP_Tuto_C|GetText_Crouch _returnvalue) "Hidden")
  (UserInterface|Animation|PlayAnimation _returnvalue (Variables|/Game/ProjectOrigin/Final/UI/WBP_Tuto.WBP_Tuto_C|GetNightVisionFadeOut _returnvalue) 0.0 1 "Forward" 1.0 false)
  (Utilities|FlowControl|Delay 0.2)
  (Widget|SetVisibility (Variables|/Game/ProjectOrigin/Final/UI/WBP_Tuto.WBP_Tuto_C|GetText_Sprint _returnvalue) "Hidden")
  (Widget|RemovefromParent _returnvalue))

(fn ConstructionScript)