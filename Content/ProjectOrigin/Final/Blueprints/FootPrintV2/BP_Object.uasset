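; BP_Object is an object Blueprint with a trigger box and a footprint prompt widget, apparently an unfinished grabbable.
; Show adds a new WBP_FootprintDefault to the viewport, while Close removes a freshly created instance, leaving the shown one untouched.
; The box overlap only casts to BP_FirstPCharacterFinal.
; HasGrabbed starts false, and the logic setting it from the character's IsPressedF is disconnected.
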(event OnComponentBeginOverlap(Box)
  (params (OverlappedComponent :type Primitive%20Component%20Object%20Reference) (OtherActor :type Actor%20Object%20Reference) (OtherComp :type Primitive%20Component%20Object%20Reference) (OtherBodyIndex :type Integer) (bFromSweep :type Boolean) (SweepResult :type Hit%20Result%20Structure%20%28by%20ref%29))
  (Utilities|Casting|CastToBP_FirstPCharacterFinal OtherActor))

(event Custom|Show
  (bind _returnvalue (UserInterface|CreateWidget "/Game/ProjectOrigin/Final/UI/FootPrint/WBP_FootprintDefault.WBP_FootprintDefault_C"))
  (UserInterface|Viewport|AddtoViewport _returnvalue 0))

(event Custom|Close
  (bind _returnvalue (UserInterface|CreateWidget "/Game/ProjectOrigin/Final/UI/FootPrint/WBP_FootprintDefault.WBP_FootprintDefault_C"))
  (Widget|RemovefromParent _returnvalue))

(event EventBeginPlay
  (Variables|Default|SethasGrabbed false))

(event EventTick
  (params (DeltaSeconds :type Float%20%28single-precision%29)))

(fn ConstructionScript)