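; BP_Casino is a rotatable puzzle-style actor that flags success when its trigger box meets a specific part of a casino actor.
; CasinoRotation adds 180 degrees to the static mesh's relative pitch; nothing in this file calls it.
; When the Box overlaps the Plane4 component of a BP_Casino, IsSucceed is set true and printed.
; BeginPlay resets the flag, and nothing clears it when the overlap ends.
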(event OnComponentBeginOverlap(Box)
  (params (OverlappedComponent :type Primitive%20Component%20Object%20Reference) (OtherActor :type Actor%20Object%20Reference) (OtherComp :type Primitive%20Component%20Object%20Reference) (OtherBodyIndex :type Integer) (bFromSweep :type Boolean) (SweepResult :type Hit%20Result%20Structure%20%28by%20ref%29))
  ;[0 0 0] Succeed
  (bind _asbp_casino (Utilities|Casting|CastToBP_Casino OtherActor))
  (if (== (Variables|BP_Casino_C|GetPlane4 _asbp_casino) OtherComp)
    (bind _output_get (Variables|Default|SetisSucceed true))
    (Development|PrintString (Utilities|String|ToString(Boolean) _output_get))))

(event EventBeginPlay
  (bind _staticmesh (Variables|Default|GetStaticMesh))
  (Transformation|SetRelativeLocationAndRotation (Variables|Default|GetStaticMesh) (Variables|/Script/Engine.SceneComponent|GetRelativeLocation _staticmesh) (Variables|/Script/Engine.SceneComponent|GetRelativeRotation _staticmesh) false false)
  (Variables|Default|SetisSucceed false))

(fn ConstructionScript)

(fn CasinoRotation
  (bind _staticmesh (Variables|Default|GetStaticMesh))
  (bind _relativerotation (Variables|/Script/Engine.SceneComponent|GetRelativeRotation _staticmesh))
  (Transformation|SetRelativeRotation _staticmesh (Math|Rotator|MakeRotator (.roll _relativerotation) (+ (.pitch _relativerotation) 1.8e+02) (.yaw _relativerotation)) false false))