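; Stele pedestal for a footprint puzzle that displays placed pieces and runs the puzzle's ending transition.
; ShowPiece reveals piece meshes and matching widget parts and sets flags that CheckEndOfPuzzle tests; leaving the box removes the widget.
; EndPuzzleTransition is a delay-timed sequence: fade to black, teleport the player, play a cinematic, fade back, light the flame VFX, close the puzzle door, then unlock and open the main labyrinth door.
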(event OnComponentEndOverlap(Box)
  (params (OverlappedComponent :type Primitive%20Component%20Object%20Reference) (OtherActor :type Actor%20Object%20Reference) (OtherComp :type Primitive%20Component%20Object%20Reference) (OtherBodyIndex :type Integer))
  (Utilities|Casting|CastToBP_FirstPCharacterFinal OtherActor)
  (Widget|RemovefromParent (Variables|Default|GetSocleSteleWidget)))

(event Custom|EndPuzzleTransition
  (bind _maindoorref (Variables|Default|GetMainDoorRef))
  ;[1 1 1] FadeIn / TP (Door) / FadeOut /Cinematic/ FadeIn_Out / Closing Door / VFX Visibility On
  (CallFunction|FadeinFadeOut "NewEnumerator0" true false)
  (Utilities|FlowControl|Delay 1.0)
  (CallFunction|TPCharacter "NewEnumerator0")
  (CallFunction|ShowCinematic)
  (CallFunction|FadeinFadeOut "NewEnumerator0" false true)
  (Utilities|FlowControl|Delay 1.5)
  (Components|Activation|Activate (Variables|/Script/Niagara.NiagaraActor|GetNiagaraComponent (Variables|Default|GetFlameVFX)) false)
  (Utilities|FlowControl|Delay 4.5)
  (Default|CloseDoor (Variables|Default|GetPuzzleDoorRef))
  (Variables|/Game/ProjectOrigin/Final/Blueprints/Manager/BP_MainDoor.BP_MainDoor_C|SetLabyrinthUnlock _maindoorref true)
  (Utilities|FlowControl|Delay 2.0)
  (Default|OpenMainDoor _maindoorref))

(event EventBeginPlay
  (bind _returnvalue (UserInterface|CreateWidget "/Game/ProjectOrigin/Final/UI/FootPrint/WBP_FootprintDefault.WBP_FootprintDefault_C"))
  (Variables|Default|SetSocleSteleWidget _returnvalue))

(fn ConstructionScript)

(fn ShowPiece
  (params (StelePiece :type Array%20of%20EStelePiece%20Enums :default "NewEnumerator0"))
  (for _array_element StelePiece
    (switch Utilities|FlowControl|Switch|SwitchonEStelePiece _array_element
      (:NewEnumerator0
        (Rendering|SetVisibility (Variables|Default|GetPiece1) true false)
        (Variables|Default|SetPiece1IsIn true)
        (Widget|SetVisibility (Variables|/Game/ProjectOrigin/Final/UI/FootPrint/WBP_FootprintDefault.WBP_FootprintDefault_C|GetPart2 (Variables|Default|GetSocleSteleWidget)) "Visible"))
      (:NewEnumerator1
        (Rendering|SetVisibility (Variables|Default|GetPiece2) true false)
        (Variables|Default|SetPiece2IsIn true)
        (Widget|SetVisibility (Variables|/Game/ProjectOrigin/Final/UI/FootPrint/WBP_FootprintDefault.WBP_FootprintDefault_C|GetPart4 (Variables|Default|GetSocleSteleWidget)) "Visible"))
      (:NewEnumerator2
        (Rendering|SetVisibility (Variables|Default|GetPiece3) true false)
        (Variables|Default|SetPiece3IsIn true)
        (Widget|SetVisibility (Variables|/Game/ProjectOrigin/Final/UI/FootPrint/WBP_FootprintDefault.WBP_FootprintDefault_C|GetPart3 (Variables|Default|GetSocleSteleWidget)) "Visible")))))

(fn CheckEndOfPuzzle
  (return (Math|Boolean|ANDBoolean (Variables|Default|GetPiece1IsIn) (Variables|Default|GetPiece2IsIn) (Variables|Default|GetPiece3IsIn))))

(fn ShowCinematic
  (bind _returnvalue (Sequencer|Player|CreateLevelSequencePlayer (Variables|Default|GetCinematic)))
  (Sequencer|Player|Play _returnvalue :!class /Script/MovieScene.MovieSceneSequencePlayer))

(fn TPCharacter
  (params (PuzzleState :type EPuzzleStates%20Enum :default "NewEnumerator0"))
  (Transformation|SetActorLocation (Game|GetPlayerCharacter 0) (Transformation|GetActorLocation (Variables|Default|GetTPPosRef)) false false))

(fn FadeinFadeOut
  (params (PuzzleState :type EPuzzleStates%20Enum :default "NewEnumerator0") (FadeIn :type Boolean) (FadeOut :type Boolean))
  (bind _asbp_first_pcharacter_final (Utilities|Casting|CastToBP_FirstPCharacterFinal (Game|GetPlayerCharacter 0)))
  (if FadeIn
    (Default|Fadeon (Variables|/Game/ProjectOrigin/Final/Blueprints/Character/BP_FirstPCharacterFinal.BP_FirstPCharacterFinal_C|GetBlackFade _asbp_first_pcharacter_final))
    (elif FadeOut
      (Default|FadeOff (Variables|/Game/ProjectOrigin/Final/Blueprints/Character/BP_FirstPCharacterFinal.BP_FirstPCharacterFinal_C|GetBlackFade _asbp_first_pcharacter_final)))))