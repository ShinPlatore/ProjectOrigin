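; BP_FinalScene is a trigger box that runs the scripted dialogue sequence at the altar in the final scene.
; On player overlap it disables input, blends to the altar camera and slides the character along X with a timeline.
; Chained delays then activate portal and flame-eye Niagara effects, play the dialogue and show subtitles.
; After a fixed one-minute wait it restores input and view, enables sprinting and disables the box's collision.
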(event OnComponentBeginOverlap(Box)
  (params (OverlappedComponent :type Primitive%20Component%20Object%20Reference) (OtherActor :type Actor%20Object%20Reference) (OtherComp :type Primitive%20Component%20Object%20Reference) (OtherBodyIndex :type Integer) (bFromSweep :type Boolean) (SweepResult :type Hit%20Result%20Structure%20%28by%20ref%29))
  ;[1 1 1] Set Dialogue Camera
  (bind _asbp_first_pcharacter_final (Utilities|Casting|CastToBP_FirstPCharacterFinal OtherActor))
  (Input|DisableInput _asbp_first_pcharacter_final 0)
  (Variables|Default|SetisFinalTheFirst true)
  (Game|Player|SetViewTargetwithBlend (Game|GetPlayerController 0) (Variables|Default|GetCameraAutel) 2.0 "VTBlend_Linear" 0.0 false)
  (Variables|Default|SetCharacterLocation (Transformation|GetActorLocation (Game|GetPlayerCharacter 0)))
  (bind _movecharacter (Timeline|MoveToPosition Play)
    (:Update
      (Transformation|SetActorLocation (Game|GetPlayerCharacter 0) (Math|Vector|MakeVector (+ _movecharacter (.x (Variables|Default|GetCharacterLocation))) (.y (Variables|Default|GetCharacterLocation)) (.z (Variables|Default|GetCharacterLocation))) false false))
    (:Finished
      (Utilities|FlowControl|Delay 1.0)
      (Components|Activation|Activate (Variables|/Script/Niagara.NiagaraActor|GetNiagaraComponent (Variables|Default|GetFX_Portal)) false)
      (Utilities|FlowControl|Delay 0.4)
      ;[1 1 1] Activate Eye VFX
      (for _array_element (Variables|Default|GetFlameEyeRef)
        (Components|Activation|Activate (Variables|/Script/Niagara.NiagaraActor|GetNiagaraComponent _array_element) false))
      ;[1 1 1] Play Dialogue Sound & Show Subtitle's Dialogue
      (Utilities|FlowControl|Delay 0.5)
      (Audio|PlaySoundatLocation "/Game/ProjectOrigin/Final/Sounds/M_Game/Dialogue_Cue.Dialogue_Cue" (Transformation|GetActorLocation (Variables|Default|GetSoundLocation)) "0, 0, 0" 1.0 1.0 0.0 0 0 0 0)
      (bind _asbp_first_pcharacter_final_2 (Utilities|Casting|CastToBP_FirstPCharacterFinal (Game|GetPlayerCharacter 0)))
      (UserInterface|Viewport|AddtoViewport (Variables|/Game/ProjectOrigin/Final/Blueprints/Character/BP_FirstPCharacterFinal.BP_FirstPCharacterFinal_C|GetSubtilesWidget _asbp_first_pcharacter_final_2) 0)
      (Utilities|FlowControl|Delay 6e+01)
      (Input|EnableInput _asbp_first_pcharacter_final_2 0)
      (Game|Player|SetViewTargetwithBlend (Game|GetPlayerController 0) _asbp_first_pcharacter_final_2 1.0 "VTBlend_Linear" 0.0 false)
      (Variables|/Game/ProjectOrigin/Final/Blueprints/Character/BP_FirstPCharacterFinal.BP_FirstPCharacterFinal_C|SetCan%20Sprint _asbp_first_pcharacter_final_2 true)
      (Collision|SetCollisionEnabled (Variables|Default|GetBox) "NoCollision"))))

(fn ConstructionScript)