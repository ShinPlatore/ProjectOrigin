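; BP_PlateformManager runs a repeating timed cycle that randomly selects three night platforms.
; A DoN loop waits for Timer and plays a sound up to three times, with an extra sound on the third beat.
; It then shuffles NightPlatformRef, refills NightPlateCache with the first three and restarts.
; SetPlatformsState applies a night status to cached platforms but is not called here, and the Transparence loop is unwired.
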(event Custom|StartCycle
  (bind _counter (Utilities|FlowControl|DoN 3)
    (:Exit
      (Development|PrintString (Utilities|String|ToString(Integer) _counter))
      (Utilities|FlowControl|Delay (Variables|Default|GetTimer))
      (Audio|PlaySound2D "/Game/ProjectOrigin/Patrick/Sounds/NewSoundCue.NewSoundCue" 5.0 0.6 0.0 0 0)
      (if (== _counter 3)
        (Audio|PlaySound2D "/Game/ProjectOrigin/Patrick/Sounds/NewSoundCue.NewSoundCue" 5.0 2.0 0.0 0 0)
        (Utilities|FlowControl|Delay 0.2)
        (Utilities|Array|Clear (Variables|Default|GetNightPlateCache))
        (CallFunction|Reset)
        (CallFunction|StartCycle)
        (else
          (CallFunction|StartCycle))))))

(event Custom|Reset
  (bind _nightplatformref (Variables|Default|GetNightPlatformRef))
  (Utilities|Array|Shuffle _nightplatformref)
  (Utilities|Array|Add (Variables|Default|GetNightPlateCache) (Utilities|Array|Get(acopy) _nightplatformref))
  (Utilities|Array|Add (Variables|Default|GetNightPlateCache) (Utilities|Array|Get(acopy) _nightplatformref 1))
  (Utilities|Array|Add (Variables|Default|GetNightPlateCache) (Utilities|Array|Get(acopy) _nightplatformref 2))
  (Utilities|FlowControl|DoN 3) ; enters at Reset
)

(event EventBeginPlay
  (bind _counter (Utilities|FlowControl|DoN 3)
    (:Exit
      (Development|PrintString (Utilities|String|ToString(Integer) _counter))
      (Utilities|FlowControl|Delay (Variables|Default|GetTimer))
      (Audio|PlaySound2D "/Game/ProjectOrigin/Patrick/Sounds/NewSoundCue.NewSoundCue" 5.0 0.6 0.0 0 0)
      (if (== _counter 3)
        (Audio|PlaySound2D "/Game/ProjectOrigin/Patrick/Sounds/NewSoundCue.NewSoundCue" 5.0 2.0 0.0 0 0)
        (Utilities|FlowControl|Delay 0.2)
        (Utilities|Array|Clear (Variables|Default|GetNightPlateCache))
        (CallFunction|Reset)
        (CallFunction|StartCycle)
        (else
          (CallFunction|StartCycle))))))

(fn ConstructionScript)

(fn SetPlatformsState
  (params (NewParam :type Boolean))
  (for _array_element (Variables|Default|GetNightPlateCache)
    (Default|SetNightStatus _array_element NewParam)))