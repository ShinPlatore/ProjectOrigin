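; BP_MetronomeLightManagerFinal runs a repeating metronome cycle that drives a group of burning lights.
; Cycledeux switches the lights off, picks a random tick interval and resets a DoN counter fired by MetronomeCycle.
; Each delayed tick plays a sound and prints the count; after the third, a final tick switches the lights on.
; After the light duration, both events are called again to restart the cycle.
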(event Custom|MetronomeCycle
  (bind _counter (Utilities|FlowControl|DoN 3)
    (:Exit
      (Utilities|FlowControl|Delay (Variables|Default|GetTimer))
      (Audio|PlaySound2D "/Game/ProjectOrigin/Patrick/Sounds/NewSoundCue.NewSoundCue" 1e+01 1.0 0.0 0 0)
      (Development|PrintString (Utilities|String|ToString(Integer) _counter))
      (if (== _counter 3)
        (Utilities|FlowControl|Delay (Variables|Default|GetTimer))
        (Audio|PlaySound2D "/Game/ProjectOrigin/Patrick/Sounds/NewSoundCue.NewSoundCue" 1e+01 2.0 0.0 0 0)
        (for _array_element (Variables|Default|GetBurningLights)
          (Default|SwitchOn/OffBurnLight _array_element true)
          (Utilities|FlowControl|Delay (Variables|Default|GetLightDuration))
          (CallFunction|Cycledeux)
          (CallFunction|MetronomeCycle))
        (else
          (CallFunction|MetronomeCycle))))))

(event Custom|Cycledeux
  (for _array_element (Variables|Default|GetBurningLights)
    (Default|SwitchOn/OffBurnLight _array_element false))
  (Variables|Default|SetTimer (Math|Random|RandomFloatinRange (Variables|Default|GetMinRandomTimer) (Variables|Default|GetMaxRandomTimer)))
  (Utilities|FlowControl|DoN 3) ; enters at Reset
)

(fn ConstructionScript)