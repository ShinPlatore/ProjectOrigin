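; BP_MainDoor is the main door actor, built from five pairs of left and right blocks that slide apart to open.
; OpenMainDoor does nothing unless DoorComplete equals 2; it then waits three seconds and plays a timeline.
; Each timeline track drives one pair's relative X position, mirrored for the left side, with small random jitter added every update to shake the blocks as they move.
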(event Custom|OpenMainDoor
  (bind _returnvalue (Math|Random|RandomFloatinRange -1.0 1.0))
  (if (== (Variables|Default|GetDoorComplete) 2)
    (Utilities|FlowControl|Delay 3.0)
    (bind (_direction _block_1 _block_2 _block_3 _block_4 _block_5) (Timeline|Timeline Play)
      (:Update
        (Transformation|SetRelativeLocation (Variables|Default|Getbloc1Left) (Math|Vector|MakeVector (* (+ _block_1 _returnvalue) -1.0) 0.0 0.0) false false)
        (Transformation|SetRelativeLocation (Variables|Default|Getbloc1Right) (Math|Vector|MakeVector (+ _block_1 _returnvalue) 0.0 0.0) false false)
        (Transformation|SetRelativeLocation (Variables|Default|Getbloc2Left) (Math|Vector|MakeVector (* (+ _block_2 _returnvalue) -1.0) 0.0 0.0) false false)
        (Transformation|SetRelativeLocation (Variables|Default|Getbloc2Right) (Math|Vector|MakeVector (+ _block_2 _returnvalue) 0.0 0.0) false false)
        (Transformation|SetRelativeLocation (Variables|Default|Getbloc3Left) (Math|Vector|MakeVector (* (+ _block_3 _returnvalue) -1.0) 0.0 0.0) false false)
        (Transformation|SetRelativeLocation (Variables|Default|Getbloc3Right) (Math|Vector|MakeVector (+ _block_3 _returnvalue) 0.0 0.0) false false)
        (Transformation|SetRelativeLocation (Variables|Default|Getbloc4Left) (Math|Vector|MakeVector (* (+ _block_4 _returnvalue) -1.0) 0.0 0.0) false false)
        (Transformation|SetRelativeLocation (Variables|Default|Getbloc4Right) (Math|Vector|MakeVector (+ _block_4 _returnvalue) 0.0 0.0) false false)
        (Transformation|SetRelativeLocation (Variables|Default|Getbloc5Left) (Math|Vector|MakeVector (* (+ _block_5 _returnvalue) -1.0) 0.0 0.0) false false)
        (Transformation|SetRelativeLocation (Variables|Default|Getbloc5Right) (Math|Vector|MakeVector (+ _block_5 _returnvalue) 0.0 0.0) false false)))))

(fn ConstructionScript)