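; Pushable cube actor for the first-person character, with a one-time push/pull tutorial prompt.
; Entering the XAxis trigger while moving enables cube physics and sets the character's IsPushing; leaving either axis trigger clears both.
; YAxis entry only casts, as its push logic is disconnected.
; A Box trigger shows WBP_TutoFinal with timed fades; exiting re-adds it, fades out and removes it.
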(event OnComponentBeginOverlap(YAxis)
  (params (OverlappedComponent :type Primitive%20Component%20Object%20Reference) (OtherActor :type Actor%20Object%20Reference) (OtherComp :type Primitive%20Component%20Object%20Reference) (OtherBodyIndex :type Integer) (bFromSweep :type Boolean) (SweepResult :type Hit%20Result%20Structure%20%28by%20ref%29))
  (bind _asbp_first_pcharacter_final (Utilities|Casting|CastToBP_FirstPCharacterFinal OtherActor)))

(event OnComponentEndOverlap(YAxis)
  (params (OverlappedComponent :type Primitive%20Component%20Object%20Reference) (OtherActor :type Actor%20Object%20Reference) (OtherComp :type Primitive%20Component%20Object%20Reference) (OtherBodyIndex :type Integer))
  (bind _asbp_first_pcharacter_final (Utilities|Casting|CastToBP_FirstPCharacterFinal OtherActor))
  (Physics|SetSimulatePhysics (Variables|Default|GetCube) false)
  (Variables|/Game/ProjectOrigin/Final/Blueprints/Character/BP_FirstPCharacterFinal.BP_FirstPCharacterFinal_C|SetisPushing _asbp_first_pcharacter_final false))

(event OnComponentBeginOverlap(XAxis)
  (params (OverlappedComponent :type Primitive%20Component%20Object%20Reference) (OtherActor :type Actor%20Object%20Reference) (OtherComp :type Primitive%20Component%20Object%20Reference) (OtherBodyIndex :type Integer) (bFromSweep :type Boolean) (SweepResult :type Hit%20Result%20Structure%20%28by%20ref%29))
  (bind _asbp_first_pcharacter_final (Utilities|Casting|CastToBP_FirstPCharacterFinal OtherActor))
  (if (== (Variables|/Game/ProjectOrigin/Final/Blueprints/Character/BP_FirstPCharacterFinal.BP_FirstPCharacterFinal_C|GetisMoving _asbp_first_pcharacter_final) true)
    (Physics|SetSimulatePhysics (Variables|Default|GetCube) true)
    (Variables|/Game/ProjectOrigin/Final/Blueprints/Character/BP_FirstPCharacterFinal.BP_FirstPCharacterFinal_C|SetisPushing _asbp_first_pcharacter_final true)))

(event OnComponentEndOverlap(XAxis)
  (params (OverlappedComponent :type Primitive%20Component%20Object%20Reference) (OtherActor :type Actor%20Object%20Reference) (OtherComp :type Primitive%20Component%20Object%20Reference) (OtherBodyIndex :type Integer))
  (bind _asbp_first_pcharacter_final (Utilities|Casting|CastToBP_FirstPCharacterFinal OtherActor))
  (Physics|SetSimulatePhysics (Variables|Default|GetCube) false)
  (Variables|/Game/ProjectOrigin/Final/Blueprints/Character/BP_FirstPCharacterFinal.BP_FirstPCharacterFinal_C|SetisPushing _asbp_first_pcharacter_final false))

(event OnComponentBeginOverlap(Box)
  (params (OverlappedComponent :type Primitive%20Component%20Object%20Reference) (OtherActor :type Actor%20Object%20Reference) (OtherComp :type Primitive%20Component%20Object%20Reference) (OtherBodyIndex :type Integer) (bFromSweep :type Boolean) (SweepResult :type Hit%20Result%20Structure%20%28by%20ref%29))
  (Utilities|Casting|CastToBP_FirstPCharacterFinal OtherActor)
  (if (== (Variables|Default|GethasBeenDisplayed) false)
    (bind _returnvalue (UserInterface|CreateWidget "/Game/ProjectOrigin/Final/UI/WBP_TutoFinal.WBP_TutoFinal_C"))
    (UserInterface|Viewport|AddtoViewport _returnvalue 0)
    (Variables|Default|SethasBeenDisplayed true)
    (Widget|SetVisibility (Variables|/Game/ProjectOrigin/Final/UI/WBP_TutoFinal.WBP_TutoFinal_C|GetText_Crouch _returnvalue) "Hidden")
    (UserInterface|Animation|PlayAnimation _returnvalue (Variables|/Game/ProjectOrigin/Final/UI/WBP_TutoFinal.WBP_TutoFinal_C|GetPushPullFadeIn _returnvalue) 0.0 1 "Forward" 1.0 false)
    (Widget|SetVisibility (Variables|/Game/ProjectOrigin/Final/UI/WBP_TutoFinal.WBP_TutoFinal_C|GetText_PushPull _returnvalue) "Visible")
    (Utilities|FlowControl|Delay 5.0)
    (UserInterface|Animation|PlayAnimation _returnvalue (Variables|/Game/ProjectOrigin/Final/UI/WBP_TutoFinal.WBP_TutoFinal_C|GetPushPullFadeOut _returnvalue) 0.0 1 "Forward" 1.0 false)
    (Utilities|FlowControl|Delay 1.0)
    (Widget|SetVisibility (Variables|/Game/ProjectOrigin/Final/UI/WBP_TutoFinal.WBP_TutoFinal_C|GetText_PushPull _returnvalue) "Hidden")
    (Widget|RemovefromParent _returnvalue)))

(event OnComponentEndOverlap(Box)
  (params (OverlappedComponent :type Primitive%20Component%20Object%20Reference) (OtherActor :type Actor%20Object%20Reference) (OtherComp :type Primitive%20Component%20Object%20Reference) (OtherBodyIndex :type Integer))
  (Utilities|Casting|CastToBP_FirstPCharacterFinal OtherActor)
  (UserInterface|Viewport|AddtoViewport (stale OnComponentBeginOverlap(Box) _returnvalue) 0)
  (UserInterface|Animation|PlayAnimation (stale OnComponentBeginOverlap(Box) _returnvalue) (Variables|/Game/ProjectOrigin/Final/UI/WBP_TutoFinal.WBP_TutoFinal_C|GetPushPullFadeOut (stale OnComponentBeginOverlap(Box) _returnvalue)) 0.0 1 "Forward" 1.0 false)
  (Utilities|FlowControl|Delay 1.0)
  (Widget|SetVisibility (Variables|/Game/ProjectOrigin/Final/UI/WBP_TutoFinal.WBP_TutoFinal_C|GetText_PushPull (stale OnComponentBeginOverlap(Box) _returnvalue)) "Hidden")
  (Widget|RemovefromParent (stale OnComponentBeginOverlap(Box) _returnvalue)))

(event EventBeginPlay
  (Development|SetHiddeninGame (Variables|Default|GetWidget) true false))

(fn ConstructionScript)