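; BP_BurningSpotLight is a puzzle spotlight that burns the player character with sun damage.
; While active, Tick fires debug-drawn Camera-channel line traces to 61 component points, calling TakeSunDamage on the first player hit.
; RotateNewAngle toggles the light's pitch forward or back through a timeline chosen by its Blue, Red or Yellow puzzle state.
; SwitchOnOffBurnLight sets damage and visibility together; OtherPuzzle lights start off.
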(event Custom|RotateNewAngle
  (switch Utilities|FlowControl|Switch|SwitchonESpotLightState (Variables|Default|GetSpotLightState)
    (:NewEnumerator0
      (Utilities|FlowControl|FlipFlop
        (:A
          (bind _0_to_90 (Timeline|Timeline Play)
            (:Update
              (Transformation|SetRelativeRotation (Variables|Default|GetSpotLight) (Math|Rotator|MakeRotator 0.0 _0_to_90 0.0) false false))))
        (:B
          (Timeline|Timeline Reverse))))
    (:NewEnumerator1
      (Utilities|FlowControl|FlipFlop
        (:A
          (bind _newtrack_0 (Timeline|Down%20To%20Up Play)
            (:Update
              (Transformation|SetRelativeRotation (Variables|Default|GetSpotLight) (Math|Rotator|MakeRotator 0.0 _newtrack_0 0.0) false false))))
        (:B
          (Timeline|Down%20To%20Up Reverse))))
    (:NewEnumerator3
      (Utilities|FlowControl|FlipFlop
        (:A
          (bind _newtrack_0_2 (Timeline|YellowTimeline Play)
            (:Update
              (Transformation|SetRelativeRotation (Variables|Default|GetSpotLight) (Math|Rotator|MakeRotator 0.0 _newtrack_0_2 0.0) false false))))
        (:B
          (Timeline|YellowTimeline Reverse))))))

(event EventBeginPlay
  (Variables|Default|SetArray (Utilities|Array|MakeArray (Variables|Default|Get1) (Variables|Default|Get2) (Variables|Default|Get3) (Variables|Default|Get4) (Variables|Default|Get5) (Variables|Default|Get6) (Variables|Default|Get7) (Variables|Default|Get8) (Variables|Default|Get9) (Variables|Default|Get10) (Variables|Default|Get11) (Variables|Default|Get12) (Variables|Default|Get13) (Variables|Default|Get14) (Variables|Default|Get15) (Variables|Default|Get16) (Variables|Default|Get17) (Variables|Default|Get18) (Variables|Default|Get19) (Variables|Default|Get20) (Variables|Default|Get21) (Variables|Default|Get22) (Variables|Default|Get23) (Variables|Default|Get24) (Variables|Default|Get25) (Variables|Default|Get26) (Variables|Default|Get27) (Variables|Default|Get28) (Variables|Default|Get29) (Variables|Default|Get30) (Variables|Default|Get31) (Variables|Default|Get32) (Variables|Default|Get33) (Variables|Default|Get34) (Variables|Default|Get35) (Variables|Default|Get36) (Variables|Default|Get37) (Variables|Default|Get38) (Variables|Default|Get39) (Variables|Default|Get40) (Variables|Default|Get41) (Variables|Default|Get42) (Variables|Default|Get43) (Variables|Default|Get44) (Variables|Default|Get45) (Variables|Default|Get46) (Variables|Default|Get47) (Variables|Default|Get48) (Variables|Default|Get49) (Variables|Default|Get50) (Variables|Default|Get51) (Variables|Default|Get52) (Variables|Default|Get53) (Variables|Default|Get54) (Variables|Default|Get55) (Variables|Default|Get56) (Variables|Default|Get57) (Variables|Default|Get58) (Variables|Default|Get59) (Variables|Default|Get60) (Variables|Default|Get61)))
  (bind _asbp_first_pcharacter_patrick (Utilities|Casting|CastToBP_FirstPCharacterPatrick (Game|GetPlayerCharacter 0)))
  (Variables|Default|SetAs%20BP%20First%20PCharacter%20Patrick _asbp_first_pcharacter_patrick)
  (if (Utilities|Enum|Equal(Enum) (Variables|Default|GetSpotLightState) "NewEnumerator2")
    (Variables|Default|SetIsActive false)
    (Rendering|SetVisibility (Variables|Default|GetSpotLight) false false)))

(event EventTick
  (params (DeltaSeconds :type Float%20%28single-precision%29))
  (bind _as_bp_first_pcharacter_patrick (Variables|Default|GetAs%20BP%20First%20PCharacter%20Patrick))
  (if (Variables|Default|GetIsActive)
    (bind _array_element (Utilities|Array|ForEachLoopwithBreak (Variables|Default|GetArray) :!label _label)
      (:LoopBody
        (bind _outhit (Collision|LineTraceByChannel (Transformation|GetActorLocation self) (Transformation|GetWorldLocation _array_element) "TraceTypeQuery2" false 0 "ForOneFrame"))
        (if (== (.hitactor _outhit) _as_bp_first_pcharacter_patrick)
          (Default|TakeSunDamage _as_bp_first_pcharacter_patrick)
          (goto _label Break))))))

(fn ConstructionScript)

(fn SwitchOn/OffBurnLight
  (params (NewParam :type Boolean))
  (Variables|Default|SetIsActive NewParam)
  (Rendering|SetVisibility (Variables|Default|GetSpotLight) NewParam false))