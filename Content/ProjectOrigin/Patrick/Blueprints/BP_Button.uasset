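; BP_Button is an in-world button that shows its state by swapping the material on its cube mesh.
; A box trigger sets InRange and switches between collide and base materials as the first-person character enters or leaves.
; The ChangeIntoTriggerColor event flashes the trigger material, then after a short delay restores the material matching the current InRange state.
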(event OnComponentBeginOverlap(Box)
  (params (OverlappedComponent :type Primitive%20Component%20Object%20Reference) (OtherActor :type Actor%20Object%20Reference) (OtherComp :type Primitive%20Component%20Object%20Reference) (OtherBodyIndex :type Integer) (bFromSweep :type Boolean) (SweepResult :type Hit%20Result%20Structure%20%28by%20ref%29))
  ;[0 0 0 1 25] Button Behavior
  (Utilities|Casting|CastToBP_FirstPCharacterPatrick OtherActor)
  (Variables|Default|SetInRange true)
  (Rendering|Material|SetMaterial (Variables|Default|GetCube) 0 "/Game/ProjectOrigin/Patrick/Mat/M_ButtonCollide.M_ButtonCollide"))

(event OnComponentEndOverlap(Box)
  (params (OverlappedComponent :type Primitive%20Component%20Object%20Reference) (OtherActor :type Actor%20Object%20Reference) (OtherComp :type Primitive%20Component%20Object%20Reference) (OtherBodyIndex :type Integer))
  ;[0 0 0 1 25] Button Behavior
  (Utilities|Casting|CastToBP_FirstPCharacterPatrick OtherActor)
  (Variables|Default|SetInRange false)
  (Rendering|Material|SetMaterial (Variables|Default|GetCube) 0 "/Game/ProjectOrigin/Patrick/Mat/M_ButtonBase.M_ButtonBase"))

(event Custom|ChangeIntoTriggerColor
  (bind _cube (Variables|Default|GetCube))
  ;[0 0 0 1 25] Button Behavior
  (Rendering|Material|SetMaterial (Variables|Default|GetCube) 0 "/Game/ProjectOrigin/Patrick/Mat/M_ButtonTrigger.M_ButtonTrigger")
  (Utilities|FlowControl|Delay 0.5)
  (if (Variables|Default|GetInRange)
    (Rendering|Material|SetMaterial _cube 0 "/Game/ProjectOrigin/Patrick/Mat/M_ButtonCollide.M_ButtonCollide")
    (else
      (Rendering|Material|SetMaterial _cube 0 "/Game/ProjectOrigin/Patrick/Mat/M_ButtonBase.M_ButtonBase"))))

(fn ConstructionScript)