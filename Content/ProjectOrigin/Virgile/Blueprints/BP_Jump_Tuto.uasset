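; Tutorial trigger actor that shows the jump hint the first time the first-person character enters its box.
; On begin overlap it creates a shared WBP_Tuto widget, shows only the jump text, and fades it in, then out on a timer before removing it.
; On end overlap it re-adds the widget to play the fade-out, then removes it and destroys itself.
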(event OnComponentBeginOverlap(Box)
  (params (OverlappedComponent :type Primitive%20Component%20Object%20Reference) (OtherActor :type Actor%20Object%20Reference) (OtherComp :type Primitive%20Component%20Object%20Reference) (OtherBodyIndex :type Integer) (bFromSweep :type Boolean) (SweepResult :type Hit%20Result%20Structure%20%28by%20ref%29))
  (Utilities|Casting|CastToBP_FirstPersonCharacter OtherActor)
  (if (== (Variables|Default|GethasBeenDisplayed) false)
    (bind _returnvalue (UserInterface|CreateWidget "/Game/ProjectOrigin/Virgile/UI/WBP_Tuto.WBP_Tuto_C"))
    (UserInterface|Viewport|AddtoViewport _returnvalue 0)
    (Variables|Default|SethasBeenDisplayed true)
    (Widget|SetVisibility (Variables|/Game/ProjectOrigin/Virgile/UI/WBP_Tuto.WBP_Tuto_C|GetText_PushPull _returnvalue) "Hidden")
    (UserInterface|Animation|PlayAnimation _returnvalue (Variables|/Game/ProjectOrigin/Virgile/UI/WBP_Tuto.WBP_Tuto_C|GetJumpFadeIn _returnvalue) 0.0 1 "Forward" 1.0 false)
    (Widget|SetVisibility (Variables|/Game/ProjectOrigin/Virgile/UI/WBP_Tuto.WBP_Tuto_C|GetText_Jump _returnvalue) "Visible")
    (Utilities|FlowControl|Delay 5.0)
    (UserInterface|Animation|PlayAnimation _returnvalue (Variables|/Game/ProjectOrigin/Virgile/UI/WBP_Tuto.WBP_Tuto_C|GetJumpFadeOut _returnvalue) 0.0 1 "Forward" 1.0 false)
    (Utilities|FlowControl|Delay 1.0)
    (Widget|SetVisibility (Variables|/Game/ProjectOrigin/Virgile/UI/WBP_Tuto.WBP_Tuto_C|GetText_Jump _returnvalue) "Hidden")
    (Widget|RemovefromParent _returnvalue)))

(event OnComponentEndOverlap(Box)
  (params (OverlappedComponent :type Primitive%20Component%20Object%20Reference) (OtherActor :type Actor%20Object%20Reference) (OtherComp :type Primitive%20Component%20Object%20Reference) (OtherBodyIndex :type Integer))
  (Utilities|Casting|CastToBP_FirstPersonCharacter OtherActor)
  (UserInterface|Viewport|AddtoViewport (stale OnComponentBeginOverlap(Box) _returnvalue) 0)
  (UserInterface|Animation|PlayAnimation (stale OnComponentBeginOverlap(Box) _returnvalue) (Variables|/Game/ProjectOrigin/Virgile/UI/WBP_Tuto.WBP_Tuto_C|GetJumpFadeOut (stale OnComponentBeginOverlap(Box) _returnvalue)) 0.0 1 "Forward" 1.0 false)
  (Utilities|FlowControl|Delay 1.0)
  (Widget|SetVisibility (Variables|/Game/ProjectOrigin/Virgile/UI/WBP_Tuto.WBP_Tuto_C|GetText_Jump (stale OnComponentBeginOverlap(Box) _returnvalue)) "Hidden")
  (Widget|RemovefromParent (stale OnComponentBeginOverlap(Box) _returnvalue))
  (Actor|DestroyActor))

(fn ConstructionScript)