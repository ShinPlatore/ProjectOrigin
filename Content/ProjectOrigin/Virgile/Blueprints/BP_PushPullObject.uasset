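; BP_PushPullObject is a cube the first-person character can push, with a tutorial prompt for push/pull.
; Overlapping its XAxis or YAxis trigger while moving enables cube physics and sets the character's IsPushing flag; leaving reverses both.
; A separate Box trigger creates WBP_Tuto and fades the push/pull text in and out, setting HasBeenDisplayed only after the delays finish.
; Its own Widget component is hidden on BeginPlay.
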(event OnComponentBeginOverlap(YAxis)
  (params (OverlappedComponent :type Primitive%20Component%20Object%20Reference) (OtherActor :type Actor%20Object%20Reference) (OtherComp :type Primitive%20Component%20Object%20Reference) (OtherBodyIndex :type Integer) (bFromSweep :type Boolean) (SweepResult :type Hit%20Result%20Structure%20%28by%20ref%29))
  (bind _asbp_first_person_character (Utilities|Casting|CastToBP_FirstPersonCharacter OtherActor))
  (if (== (Variables|/Game/ProjectOrigin/Virgile/Blueprints/BP_FirstPersonCharacter.BP_FirstPersonCharacter_C|GetisMoving _asbp_first_person_character) true)
    (Physics|SetSimulatePhysics (Variables|Default|GetCube) true)
    (Variables|/Game/ProjectOrigin/Virgile/Blueprints/BP_FirstPersonCharacter.BP_FirstPersonCharacter_C|SetisPushing _asbp_first_person_character true)))

(event OnComponentEndOverlap(YAxis)
  (params (OverlappedComponent :type Primitive%20Component%20Object%20Reference) (OtherActor :type Actor%20Object%20Reference) (OtherComp :type Primitive%20Component%20Object%20Reference) (OtherBodyIndex :type Integer))
  (bind _asbp_first_person_character (Utilities|Casting|CastToBP_FirstPersonCharacter OtherActor))
  (Physics|SetSimulatePhysics (Variables|Default|GetCube) false)
  (Variables|/Game/ProjectOrigin/Virgile/Blueprints/BP_FirstPersonCharacter.BP_FirstPersonCharacter_C|SetisPushing _asbp_first_person_character false))

(event OnComponentBeginOverlap(XAxis)
  (params (OverlappedComponent :type Primitive%20Component%20Object%20Reference) (OtherActor :type Actor%20Object%20Reference) (OtherComp :type Primitive%20Component%20Object%20Reference) (OtherBodyIndex :type Integer) (bFromSweep :type Boolean) (SweepResult :type Hit%20Result%20Structure%20%28by%20ref%29))
  (bind _asbp_first_person_character (Utilities|Casting|CastToBP_FirstPersonCharacter OtherActor))
  (if (== (Variables|/Game/ProjectOrigin/Virgile/Blueprints/BP_FirstPersonCharacter.BP_FirstPersonCharacter_C|GetisMoving _asbp_first_person_character) true)
    (Physics|SetSimulatePhysics (Variables|Default|GetCube) true)
    (Variables|/Game/ProjectOrigin/Virgile/Blueprints/BP_FirstPersonCharacter.BP_FirstPersonCharacter_C|SetisPushing _asbp_first_person_character true)))

(event OnComponentEndOverlap(XAxis)
  (params (OverlappedComponent :type Primitive%20Component%20Object%20Reference) (OtherActor :type Actor%20Object%20Reference) (OtherComp :type Primitive%20Component%20Object%20Reference) (OtherBodyIndex :type Integer))
  (bind _asbp_first_person_character (Utilities|Casting|CastToBP_FirstPersonCharacter OtherActor))
  (Physics|SetSimulatePhysics (Variables|Default|GetCube) false)
  (Variables|/Game/ProjectOrigin/Virgile/Blueprints/BP_FirstPersonCharacter.BP_FirstPersonCharacter_C|SetisPushing _asbp_first_person_character false))

(event OnComponentBeginOverlap(Box)
  (params (OverlappedComponent :type Primitive%20Component%20Object%20Reference) (OtherActor :type Actor%20Object%20Reference) (OtherComp :type Primitive%20Component%20Object%20Reference) (OtherBodyIndex :type Integer) (bFromSweep :type Boolean) (SweepResult :type Hit%20Result%20Structure%20%28by%20ref%29))
  (Utilities|Casting|CastToBP_FirstPersonCharacter OtherActor)
  (if (not (Variables|Default|GethasBeenDisplayed))
    (bind _returnvalue (UserInterface|CreateWidget "/Game/ProjectOrigin/Virgile/UI/WBP_Tuto.WBP_Tuto_C"))
    (Widget|SetVisibility (Variables|/Game/ProjectOrigin/Virgile/UI/WBP_Tuto.WBP_Tuto_C|GetText_PickUp _returnvalue) "Hidden")
    (UserInterface|Animation|PlayAnimation _returnvalue (Variables|/Game/ProjectOrigin/Virgile/UI/WBP_Tuto.WBP_Tuto_C|GetPushPullFadeIn _returnvalue) 0.0 1 "Forward" 1.0 false)
    (Widget|SetVisibility (Variables|/Game/ProjectOrigin/Virgile/UI/WBP_Tuto.WBP_Tuto_C|GetText_PushPull _returnvalue) "Visible")
    (Utilities|FlowControl|Delay 7.0)
    (UserInterface|Animation|PlayAnimation _returnvalue (Variables|/Game/ProjectOrigin/Virgile/UI/WBP_Tuto.WBP_Tuto_C|GetPushPullFadeOut _returnvalue) 0.0 1 "Forward" 1.0 false)
    (Utilities|FlowControl|Delay 1.0)
    (Widget|SetVisibility (Variables|/Game/ProjectOrigin/Virgile/UI/WBP_Tuto.WBP_Tuto_C|GetText_PushPull _returnvalue) "Hidden")
    (Variables|Default|SethasBeenDisplayed true)))

(event OnComponentEndOverlap(Box)
  (params (OverlappedComponent :type Primitive%20Component%20Object%20Reference) (OtherActor :type Actor%20Object%20Reference) (OtherComp :type Primitive%20Component%20Object%20Reference) (OtherBodyIndex :type Integer))
  (Utilities|Casting|CastToBP_FirstPersonCharacter OtherActor))

(event EventBeginPlay
  (Development|SetHiddeninGame (Variables|Default|GetWidget) true false))

(fn ConstructionScript)