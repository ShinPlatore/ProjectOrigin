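; A rotatable burning spotlight that deals sun damage to the player character caught in its traces.
; Every tick it fires debug-drawn Camera-channel line traces from the actor to an array of 61 components set at BeginPlay, breaking after the first player hit.
; RotateNewAngle uses FlipFlops to play or reverse a timeline that pitches the SpotLight, with IsRedPuzzle selecting which timeline drives it.
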(event Custom|RotateNewAngle
  (if (Variables|Default|GetIsRedPuzzle)
    (Utilities|FlowControl|FlipFlop
      (:A
        (bind _newtrack_0 (Timeline|Down%20To%20Up Play)
          (:Update
            (Transformation|SetRelativeRotation (Variables|Default|GetSpotLight) (Math|Rotator|MakeRotator 0.0 _newtrack_0 0.0) false false))))
      (:B
        (Timeline|Down%20To%20Up Reverse)))
    (else
      (Utilities|FlowControl|FlipFlop
        (:A
          (bind _0_to_90 (Timeline|Timeline Play)
            (:Update
              (Transformation|SetRelativeRotation (Variables|Default|GetSpotLight) (Math|Rotator|MakeRotator 0.0 _0_to_90 0.0) false false))))
        (:B
          (Timeline|Timeline Reverse))))))

(event EventBeginPlay
  (Variables|Default|SetArray (Utilities|Array|MakeArray (Variables|Default|Get1) (Variables|Default|Get2) (Variables|Default|Get3) (Variables|Default|Get4) (Variables|Default|Get5) (Variables|Default|Get6) (Variables|Default|Get7) (Variables|Default|Get8) (Variables|Default|Get9) (Variables|Default|Get10) (Variables|Default|Get11) (Variables|Default|Get12) (Variables|Default|Get13) (Variables|Default|Get14) (Variables|Default|Get15) (Variables|Default|Get16) (Variables|Default|Get17) (Variables|Default|Get18) (Variables|Default|Get19) (Variables|Default|Get20) (Variables|Default|Get21) (Variables|Default|Get22) (Variables|Default|Get23) (Variables|Default|Get24) (Variables|Default|Get25) (Variables|Default|Get26) (Variables|Default|Get27) (Variables|Default|Get28) (Variables|Default|Get29) (Variables|Default|Get30) (Variables|Default|Get31) (Variables|Default|Get32) (Variables|Default|Get33) (Variables|Default|Get34) (Variables|Default|Get35) (Variables|Default|Get36) (Variables|Default|Get37) (Variables|Default|Get38) (Variables|Default|Get39) (Variables|Default|Get40) (Variables|Default|Get41) (Variables|Default|Get42) (Variables|Default|Get43) (Variables|Default|Get44) (Variables|Default|Get45) (Variables|Default|Get46) (Variables|Default|Get47) (Variables|Default|Get48) (Variables|Default|Get49) (Variables|Default|Get50) (Variables|Default|Get51) (Variables|Default|Get52) (Variables|Default|Get53) (Variables|Default|Get54) (Variables|Default|Get55) (Variables|Default|Get56) (Variables|Default|Get57) (Variables|Default|Get58) (Variables|Default|Get59) (Variables|Default|Get60) (Variables|Default|Get61)))
  (Utilities|Casting|CastToBP_FirstPCharacterVirgile (Game|GetPlayerCharacter 0)))

(event EventTick
  (params (DeltaSeconds :type Float%20%28single-precision%29))
  (bind _array_element (Utilities|Array|ForEachLoopwithBreak (Variables|Default|GetArray) :!label _label)
    (:LoopBody
      (bind _outhit (Collision|LineTraceByChannel (Transformation|GetActorLocation self) (Transformation|GetWorldLocation _array_element) "TraceTypeQuery2" false 0 "ForOneFrame"))
      (bind _asbp_first_pcharacter_virgile (Utilities|Casting|CastToBP_FirstPCharacterVirgile (.hitactor _outhit)))
      (Default|TakeSunDamage _asbp_first_pcharacter_virgile)
      (goto _label Break))))

(fn ConstructionScript)