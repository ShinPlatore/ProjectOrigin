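; Trigger actor that manages a referenced lights actor, restoring it to a spawn point at BeginPlay by unhiding it, setting physics-only collision on its cube and teleporting it.
; When BP_FirstPCharacterVirgile overlaps the box, the trigger teleports itself to a Point transform.
; If that player's health is zero or below at that moment, the lights return to the spawn point after a short delay.
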(event OnComponentBeginOverlap(Box)
  (params (OverlappedComponent :type Primitive%20Component%20Object%20Reference) (OtherActor :type Actor%20Object%20Reference) (OtherComp :type Primitive%20Component%20Object%20Reference) (OtherBodyIndex :type Integer) (bFromSweep :type Boolean) (SweepResult :type Hit%20Result%20Structure%20%28by%20ref%29))
  (bind _asbp_first_pcharacter_virgile (Utilities|Casting|CastToBP_FirstPCharacterVirgile OtherActor))
  (Transformation|SetActorTransform (Variables|Default|GetPoint))
  (if (<= (Variables|/Game/ProjectOrigin/Virgile/Blueprints/Character/BP_FirstPCharacterVirgile.BP_FirstPCharacterVirgile_C|GetHealthBar _asbp_first_pcharacter_virgile) 0.0)
    (Utilities|FlowControl|Delay 2.0)
    (Transformation|SetActorTransform (Variables|Default|GetLightsREF) (Variables|Default|GetSpawnPoint))))

(event Custom|Reset
  (bind _lightsref (Variables|Default|GetLightsREF))
  (Rendering|SetActorHiddenInGame _lightsref false)
  (Collision|SetCollisionEnabled (Variables|/Game/ProjectOrigin/Virgile/Blueprints/Footprint/BP_Lights.BP_Lights_C|GetCube _lightsref) "PhysicsOnly")
  (Transformation|SetActorTransform (Variables|Default|GetLightsREF) (Variables|Default|GetSpawnPoint)))

(event EventBeginPlay
  (CallFunction|Reset))

(fn ConstructionScript)