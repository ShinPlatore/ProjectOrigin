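; BP_FakePrint5 is a fake footprint actor whose plane and static mesh are only visible in game while the player has night vision.
; It hides both components on BeginPlay.
; Every Tick it calls Display, which casts the player character to BP_FirstPCharacterVirgile and shows or hides the components according to its HasNightVision flag.
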(event Custom|Display
  (bind _asbp_first_pcharacter_virgile (Utilities|Casting|CastToBP_FirstPCharacterVirgile (Game|GetPlayerCharacter 0)))
  (if (== (Variables|/Game/ProjectOrigin/Virgile/Blueprints/Character/BP_FirstPCharacterVirgile.BP_FirstPCharacterVirgile_C|GethasNightVision _asbp_first_pcharacter_virgile) true)
    (Development|SetHiddeninGame (Variables|Default|GetPlane) false false)
    (else
      (Development|SetHiddeninGame (Variables|Default|GetPlane) true false))))

(event EventBeginPlay
  (Development|SetHiddeninGame (Variables|Default|GetPlane) true false))

(event EventTick
  (params (DeltaSeconds :type Float%20%28single-precision%29))
  (CallFunction|Display))

(fn ConstructionScript)