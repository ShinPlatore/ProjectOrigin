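; BP_Timer is a minimal timer Blueprint that counts Seconds and Minutes and shows them as debug text.
; Tick adds one to Seconds every frame, independent of delta time.
; Once Seconds exceeds 59, each tick also increments Minutes and prints both values, with Minutes in red.
; Seconds is never reset, so Minutes keeps rising every frame after that threshold.
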(event EventTick
  (params (DeltaSeconds :type Float%20%28single-precision%29))
  (bind _output_get (Variables|Default|SetSeconds (+ (Variables|Default|GetSeconds) 1)))
  (if (> (Variables|Default|GetSeconds) 59)
    (bind _output_get_2 (Variables|Default|SetMinutes (+ (Variables|Default|GetMinutes) 1)))
    (Development|PrintString (Utilities|String|ToString(Integer) _output_get))
    (Development|PrintString (Utilities|String|ToString(Integer) _output_get_2) true true "(R=1.000000,G=0.070175,B=0.000000,A=1.000000)")))

(fn ConstructionScript)