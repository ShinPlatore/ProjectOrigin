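; Trigger volume that switches levels when the BP_FirstPCharacterVirgile character overlaps its box.
; If the character has succeeded, it plays a black fade widget, waits briefly, stores its SpawnPoint in the BP_SpawnPoints game instance and opens ThirdPersonMap.
; Otherwise it opens the Footprint level, or destroys the character if the game instance's HasBeenFootprint flag is already set.
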(event OnComponentBeginOverlap(Box)
  (params (OverlappedComponent :type Primitive%20Component%20Object%20Reference) (OtherActor :type Actor%20Object%20Reference) (OtherComp :type Primitive%20Component%20Object%20Reference) (OtherBodyIndex :type Integer) (bFromSweep :type Boolean) (SweepResult :type Hit%20Result%20Structure%20%28by%20ref%29))
  (bind _asbp_first_pcharacter_virgile (Utilities|Casting|CastToBP_FirstPCharacterVirgile OtherActor))
  (if (== (Variables|/Game/ProjectOrigin/Virgile/Blueprints/Character/BP_FirstPCharacterVirgile.BP_FirstPCharacterVirgile_C|GethasSucceed _asbp_first_pcharacter_virgile) true)
    (bind _returnvalue (UserInterface|CreateWidget "/Game/ProjectOrigin/Virgile/UI/WBP_BlackFade.WBP_BlackFade_C"))
    (UserInterface|Viewport|AddtoViewport _returnvalue 0)
    (UserInterface|Animation|PlayAnimation _returnvalue (Variables|/Game/ProjectOrigin/Virgile/UI/WBP_BlackFade.WBP_BlackFade_C|GetFadeIn _returnvalue) 0.0 1 "Forward" 1.0 false)
    (Utilities|FlowControl|Delay 1.0)
    (bind _asbp_spawn_points (Utilities|Casting|CastToBP_SpawnPoints (Game|GetGameInstance)))
    (Variables|/Game/ProjectOrigin/Virgile/Blueprints/BP_SpawnPoints.BP_SpawnPoints_C|SetSpawnPointFootPrint _asbp_spawn_points (Variables|Default|GetSpawnPoint))
    (Game|OpenLevel(byObjectReference) "/Game/ProjectOrigin/Virgile/Maps/ThirdPersonMap.ThirdPersonMap")
    (elif (== (Variables|/Game/ProjectOrigin/Virgile/Blueprints/BP_SpawnPoints.BP_SpawnPoints_C|GethasBeenFootprint (.AsBP%20Spawn%20Points (Utilities|Casting|CastToBP_SpawnPoints (Game|GetGameInstance)))) true)
      (Actor|DestroyActor _asbp_first_pcharacter_virgile)
      (else
        (Game|OpenLevel(byObjectReference) "/Game/ProjectOrigin/Virgile/Maps/Footprint.Footprint")))))

(fn ConstructionScript)