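; Player controller that sets up first-person Enhanced Input and opens or closes the pause menu, apparently used for key selection.
; On BeginPlay it adds the default FPS mapping context, retries each tick until player-mappable key mappings exist, then prints each action name and key.
; CreateKeySelector shows the pause menu with cursor and Game-and-UI input.
; RemoveKeySelector removes it and hides the cursor, without resetting input mode.
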(event Custom|CreateKeySelector
  (bind _returnvalue (UserInterface|CreateWidget "/Game/ProjectOrigin/Virgile/UI/WBP_PauseMenu.WBP_PauseMenu_C"))
  (bind _output_get (Variables|Default|SetPauseMenuREF _returnvalue))
  (UserInterface|Viewport|AddtoViewport _output_get 0)
  (Variables|Default|SetbShowMouseCursor true)
  (Input|SetInputModeGameandUI self _output_get "DoNotLock" true false))

(event Custom|RemoveKeySelector
  (bind _pausemenuref (Variables|Default|GetPauseMenuREF)
    (:then
      (Widget|RemovefromParent _pausemenuref)
      (Variables|Default|SetbShowMouseCursor false))
    (:else)))

(event EventBeginPlay
  (Input|AddMappingContext (PlayerController|LocalPlayerSubsystems|GetEnhancedInputLocalPlayerSubsystem) "/Game/ProjectOrigin/Virgile/InputFirstPerson/IMC_DefaultFPS.IMC_DefaultFPS" 0 "(bIgnoreAllPressedKeysUntilRelease=True,bForceImmediately=False)")
  (if (Math|Conversions|ToBoolean(Integer) (Utilities|Array|Length (Class|EnhancedInputSubsystemInterface|GetAllPlayerMappableActionKeyMappings (PlayerController|LocalPlayerSubsystems|GetEnhancedInputLocalPlayerSubsystem)))) :!label _label
    (bind _output_get (Variables|Default|SetMappings (Class|EnhancedInputSubsystemInterface|GetAllPlayerMappableActionKeyMappings (PlayerController|LocalPlayerSubsystems|GetEnhancedInputLocalPlayerSubsystem))))
    (for _array_element _output_get
      (Development|PrintString (Utilities|String|Append (Utilities|String|ToString(Name) (.name (.playermappableoptions _array_element))) "[" "]" (Utilities|String|ToString(Text) (Class|KismetInputLibrary|KeyGetDisplayName (.key _array_element) true)))))
    (else
      (Utilities|FlowControl|DelayUntilNextTick)
      (goto _label))))

(fn ConstructionScript)